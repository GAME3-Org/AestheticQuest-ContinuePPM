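; BP_InteractionArea is an interaction area actor that relays focus changes to the parent actor it is attached to.
; ToggleFocus stores the focused state and passes it to the parent through an interface message.
; It then gets the parent's interaction widget through another message and shows it while focused, hiding it otherwise.
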(event Custom|ToggleFocus
  (params (Focused :type Boolean))
  (bind _output_get (Variables|Default|SetFocused Focused))
  (Class|BPIInteraction|InterfaceToggleFocus(Message) (Actor|GetParentActor) (Variables|Default|GetFocused))
  (bind _refwidget (Class|BPIInteraction|GetInteractionWidgetRef(Message) (Actor|GetParentActor)))
  (Development|SetHiddeninGame _refwidget (not (Variables|Default|GetFocused)) false))

(fn ConstructionScript)