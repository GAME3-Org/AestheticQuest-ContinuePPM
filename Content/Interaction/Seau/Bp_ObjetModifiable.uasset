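; Modifiable interaction object whose Objet component changes custom depth stencil value when touched by a BP_ProjectileRender.
; Overlap and Hit events share one path that prints the overlapping actor's name for debugging and sets the stencil to 2 if its class matches the projectile.
; Paintby and the widget and pickup functions are empty stubs.
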(event EventBeginPlay)

(event Collision|EventActorBeginOverlap
  (params (OtherActor :type Actor%20Object%20Reference))
  (Development|PrintString "toucher par:")
  (Development|PrintString (Utilities|GetDisplayName OtherActor))
  (if (== (Utilities|GetClass OtherActor) "/Game/Interaction/Seau/BP_ProjectileRender.BP_ProjectileRender_C")
    (Development|PrintString "toucher par:")
    (Rendering|SetCustomDepthStencilValue (Variables|Default|GetObjet) (+ (Math|Float|Truncate 0.0) 2))))

(event EventTick
  (params (DeltaSeconds :type Float%20%28single-precision%29)))

(event Collision|EventHit
  (params (MyComp :type Primitive%20Component%20Object%20Reference) (Other :type Actor%20Object%20Reference) (OtherComp :type Primitive%20Component%20Object%20Reference) (bSelfMoved :type Boolean) (HitLocation :type Vector :default "0, 0, 0") (HitNormal :type Vector :default "0, 0, 0") (NormalImpulse :type Vector :default "0, 0, 0") (Hit :type Hit%20Result%20Structure%20%28by%20ref%29))
  (Development|PrintString "toucher par:")
  (Development|PrintString (Utilities|GetDisplayName (stale Collision|EventActorBeginOverlap OtherActor)))
  (if (== (Utilities|GetClass (stale Collision|EventActorBeginOverlap OtherActor)) "/Game/Interaction/Seau/BP_ProjectileRender.BP_ProjectileRender_C")
    (Development|PrintString "toucher par:")
    (Rendering|SetCustomDepthStencilValue (Variables|Default|GetObjet) (+ (Math|Float|Truncate 0.0) 2))))

(event EventPaintby
  (params (SeauEnQuestion :type Float%20%28double-precision%29)))

(fn ConstructionScript)

(fn GetInteractionWidgetRef
  (return 0))

(fn PickUpIt
  (return ""))

(fn PickUpItem
  (return ""))