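; BP_SeauTerrain is a bucket ("seau") actor that takes one of four visual styles: neutral, BnW, Pop or Jap.
; On BeginPlay, a Sequence compares TypeOfSeau against each style number and sets the matching static mesh on the Seau component.
; The construction script is empty, so the chosen mesh is applied only at runtime, and the file has no interaction logic.
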(event EventBeginPlay
  (Utilities|FlowControl|Sequence
    (:then_0
      ;[1 1 1] SeauNeutre
      (if (== (Variables|Default|GetTypeOfSeau) 1.0)
        (Components|StaticMesh|SetStaticMesh (Variables|Default|Get%20Seau) "/Game/Interaction/Seau/SeauBase01.SeauBase01")))
    (:then_1
      ;[1 1 1] SeauBnW
      (if (== (Variables|Default|GetTypeOfSeau) 2.0)
        (Components|StaticMesh|SetStaticMesh (Variables|Default|Get%20Seau) "/Game/Interaction/Seau/SeauBase02.SeauBase02")))
    (:then_2
      ;[1 1 1] SeauPop
      (if (== (Variables|Default|GetTypeOfSeau) 3.0)
        (Components|StaticMesh|SetStaticMesh (Variables|Default|Get%20Seau) "/Game/Interaction/Seau/SeauBase03.SeauBase03")))
    (:then_3
      ;[1 1 1] SeauJap
      (if (== (Variables|Default|GetTypeOfSeau) 4.0)
        (Components|StaticMesh|SetStaticMesh (Variables|Default|Get%20Seau) "/Game/Interaction/Seau/SeauBase04.SeauBase04")))))

(event Collision|EventActorBeginOverlap
  (params (OtherActor :type Actor%20Object%20Reference)))

(event EventTick
  (params (DeltaSeconds :type Float%20%28single-precision%29)))

(fn ConstructionScript)