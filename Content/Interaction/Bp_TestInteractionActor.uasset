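; Test interactable actor that switches a point light on and off through an interaction interface, with debug prints throughout.
; Focus toggles custom depth rendering on the cube and a getter exposes its interaction widget.
; Interact calls InteractOnServer, which flips InteractToggle; its RepNotify then sets the light's visibility to match.
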(event Custom|InteractOnServer
  (Development|PrintString "ok notify" true true "(R=0.865145,G=0.000000,B=1.000000,A=1.000000)")
  (Variables|Default|SetInteractToggle (not (Variables|Default|GetInteractToggle))))

(event EventBeginPlay)

(event Collision|EventActorBeginOverlap
  (params (OtherActor :type Actor%20Object%20Reference)))

(event EventTick
  (params (DeltaSeconds :type Float%20%28single-precision%29)))

(event EventInterfaceToggleFocus
  (params (Focus :type Boolean))
  (Rendering|SetRenderCustomDepth (Variables|Default|GetCube) Focus)
  (Development|PrintString (Utilities|String|ToString(Boolean) Focus) true true "(R=1.000000,G=0.528823,B=0.000000,A=1.000000)"))

(event EventInteractInterface)

(event EventInterfaceInteract
  (Development|PrintString "ff" true true "(R=1.000000,G=0.241012,B=0.789149,A=1.000000)")
  (CallFunction|InteractonServer)
  (Development|PrintString "ca interagit ou pas ?" true true "(R=1.000000,G=0.241012,B=0.789149,A=1.000000)"))

(fn ConstructionScript)

(fn OnRepInteractToggle
  (bind _pointlight (Variables|Default|GetPointLight))
  (Development|PrintString "apeller notify" true true "(R=0.000000,G=1.000000,B=0.170053,A=1.000000)")
  (if (Variables|Default|GetInteractToggle)
    (Development|PrintString "allumer" true true "(R=0.916948,G=1.000000,B=0.000000,A=1.000000)")
    (Rendering|SetVisibility _pointlight true false)
    (else
      (Development|PrintString "pas allumer" true true "(R=1.000000,G=0.926994,B=0.000000,A=1.000000)")
      (Rendering|SetVisibility _pointlight false false))))

(fn GetInteractionWidgetRef
  (return (Variables|Default|GetWidget)))