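; Replicated interactable platform actor that moves its cube vertically with a timeline lerp.
; The MoveLift timeline starts after a short delay on BeginPlay, printing the cube's location each update.
; Interaction calls InteractOnServer to toggle InteractRep, whose OnRep calls AniamteLift, though its branch is fixed true so it only plays forward.
; Both InteractEvent and InteractEventMod switch off the cube's custom-depth rendering.
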(event Custom|AniamteLift
  (params (Up :type Boolean))
  (bind _cube (Variables|Default|GetCube))
  (if true
    (bind _newtrack_0 (Timeline|MoveLift Play)
      (:Update
        (Development|PrintString (Utilities|String|ToString(Vector) (Transformation|GetWorldLocation _cube)))
        (Transformation|SetRelativeLocation _cube (Math|Vector|Lerp(Vector) "0, 0, 0" "0.000000,0.000000,175.000000" _newtrack_0) false false)))
    (else
      (Timeline|MoveLift Reverse))))

(event Custom|InteractOnServer
  (Variables|Default|SetInteractRep (not (Variables|Default|GetInteractRep))))

(event EventBeginPlay
  (bind _cube (Variables|Default|GetCube))
  (Utilities|FlowControl|Delay 3.0)
  (bind _newtrack_0 (Timeline|MoveLift Play)
    (:Update
      (Development|PrintString (Utilities|String|ToString(Vector) (Transformation|GetWorldLocation _cube)))
      (Transformation|SetRelativeLocation _cube (Math|Vector|Lerp(Vector) "0, 0, 0" "0.000000,0.000000,175.000000" _newtrack_0) false false))))

(event Collision|EventActorBeginOverlap
  (params (OtherActor :type Actor%20Object%20Reference)))

(event EventTick
  (params (DeltaSeconds :type Float%20%28single-precision%29)))

(event EventInterfaceInteract
  (CallFunction|InteractonServer))

(event EventInteractEvent
  (Rendering|SetRenderCustomDepth (Variables|Default|GetCube) false))

(event EventInteractEventMod
  (Rendering|SetRenderCustomDepth (Variables|Default|GetCube) false))

(fn ConstructionScript)

(fn OnRepInteractRep
  (CallFunction|AniamteLift (Variables|Default|GetInteractRep)))

(fn EventInteractFocus
  (return))

(fn InteractFunction
  (params (NewParam1 :type Boolean)))